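; Post-process actor that layers toggleable screen effects, such as pixelation, fog, cel shading, water, frost, damage and night vision, onto its BasePostProcess component.
; Setup copies the bounds and settings to the component, then CheckState calls one Create function per effect.
; Each enabled effect lazily creates a dynamic material instance, adds it as a blendable and applies any parameters.
; This runs on BeginPlay, and during construction when IsEnabled; disabled effects are never explicitly removed.
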(event `self.ReceiveBeginPlay`
  (`self.Setup`)
  (`self.CheckState`))

(fn `CheckState`
  (`self.CreatePixelation` (`self.bEnablePixelation`))
  (`self.CreateFog` (`self.bEnableFog`))
  (`self.CreateCellShading` (`self.bEnableCellShader`))
  (`self.CreateWater` (`self.bEnableWater`))
  (`self.CreateDesert` (`self.bEnableDesert`))
  (`self.CreateFrost` (`self.bEnableFrost`))
  (`self.CreateDamage` (`self.bEnableDamage`))
  (`self.CreateRadiation` (`self.bEnableRadiation`))
  (`self.CreateNightVision` (`self.bEnableNightVision`)))

(fn `CreateCellShading`
  (params (bIsEnabled :type Boolean))
  (if bIsEnabled
    (`/Engine/EditorBlueprintResources/StandardMacros.IsValid` (`self.MI_CellShading`)
      (:`Is Valid`
        _)
      (:`Is Not Valid`
        (bind _returnvalue (`KismetMaterialLibrary.CreateDynamicMaterialInstance` (`self.M_CellShading`)))
        (set `self.MI_CellShading` _returnvalue)))
    (`PostProcessComponent.AddOrUpdateBlendable` (`self.BasePostProcess`) (`self.MI_CellShading`) 1.0))
  (return))

(fn `CreateDamage`
  (params (bIsEnabled :type Boolean))
  (if bIsEnabled
    (`/Engine/EditorBlueprintResources/StandardMacros.IsValid` (`self.MI_Damage`)
      (:`Is Valid`
        _)
      (:`Is Not Valid`
        (bind _returnvalue (`KismetMaterialLibrary.CreateDynamicMaterialInstance` (`self.M_Damage`)))
        (set `self.MI_Damage` _returnvalue)))
    (`PostProcessComponent.AddOrUpdateBlendable` (`self.BasePostProcess`) (`self.MI_Damage`) 1.0)
    (`MaterialInstanceDynamic.SetScalarParameterValue` (`self.MI_Damage`) "Radius" (`self.DamageRadius`))
    (`MaterialInstanceDynamic.SetScalarParameterValue` (`self.MI_Damage`) "FlickerSpeed" (`self.DamageFlickerSpeed`)))
  (return))

(fn `CreateDesert`
  (params (bIsEnabled :type Boolean))
  (if bIsEnabled
    (`/Engine/EditorBlueprintResources/StandardMacros.IsValid` (`self.MI_Desert`)
      (:`Is Valid`
        _)
      (:`Is Not Valid`
        (bind _returnvalue (`KismetMaterialLibrary.CreateDynamicMaterialInstance` (`self.M_Desert`)))
        (set `self.MI_Desert` _returnvalue)))
    (`PostProcessComponent.AddOrUpdateBlendable` (`self.BasePostProcess`) (`self.MI_Desert`) 1.0)
    (`MaterialInstanceDynamic.SetScalarParameterValue` (`self.MI_Desert`) "Sharpness" (`self.DesetSharpness`))
    (`MaterialInstanceDynamic.SetScalarParameterValue` (`self.MI_Desert`) "Distance" (`self.DesertDistance`))
    (`MaterialInstanceDynamic.SetScalarParameterValue` (`self.MI_Desert`) "HeatDistance" (`self.HeatDistance`)))
  (return))

(fn `CreateFog`
  (params (bIsEnabled :type Boolean))
  (if bIsEnabled
    (`/Engine/EditorBlueprintResources/StandardMacros.IsValid` (`self.MI_Fog`)
      (:`Is Valid`
        _)
      (:`Is Not Valid`
        (bind _returnvalue (`KismetMaterialLibrary.CreateDynamicMaterialInstance` (`self.M_Fog`)))
        (set `self.MI_Fog` _returnvalue)))
    (`PostProcessComponent.AddOrUpdateBlendable` (`self.BasePostProcess`) (`self.MI_Fog`) 1.0)
    (`MaterialInstanceDynamic.SetScalarParameterValue` (`self.MI_Fog`) "Distance" (`self.FogDistance`))
    (`MaterialInstanceDynamic.SetScalarParameterValue` (`self.MI_Fog`) "Sharpness" (`self.FogSharpness`))
    (`MaterialInstanceDynamic.SetVectorParameterValue` (`self.MI_Fog`) "FogColor" (`self.FogColor`)))
  (return))

(fn `CreateFrost`
  (params (bIsEnabled :type Boolean))
  (if bIsEnabled
    (`/Engine/EditorBlueprintResources/StandardMacros.IsValid` (`self.MI_Frost`)
      (:`Is Valid`
        _)
      (:`Is Not Valid`
        (bind _returnvalue (`KismetMaterialLibrary.CreateDynamicMaterialInstance` (`self.M_Fros`)))
        (set `self.MI_Frost` _returnvalue)))
    (`PostProcessComponent.AddOrUpdateBlendable` (`self.BasePostProcess`) (`self.MI_Frost`) 1.0)
    (`MaterialInstanceDynamic.SetScalarParameterValue` (`self.MI_Frost`) "Sharpness" (`self.FrostSharpness`))
    (`MaterialInstanceDynamic.SetScalarParameterValue` (`self.MI_Frost`) "Distance" (`self.FrostDistance`))
    (`MaterialInstanceDynamic.SetScalarParameterValue` (`self.MI_Frost`) "Radius" (`self.FrostRadius`)))
  (return))

(fn `CreateNightVision`
  (params (bIsEnabled :type Boolean))
  (if bIsEnabled
    (`/Engine/EditorBlueprintResources/StandardMacros.IsValid` (`self.MI_NightVision`)
      (:`Is Valid`
        _)
      (:`Is Not Valid`
        (bind _returnvalue (`KismetMaterialLibrary.CreateDynamicMaterialInstance` (`self.M_NightVision`)))
        (set `self.MI_NightVision` _returnvalue)))
    (`PostProcessComponent.AddOrUpdateBlendable` (`self.BasePostProcess`) (`self.MI_NightVision`) 1.0))
  (return))

(fn `CreatePixelation`
  (params (bIsEnabled :type Boolean))
  (if bIsEnabled
    (`/Engine/EditorBlueprintResources/StandardMacros.IsValid` (`self.MI_Pixelation`)
      (:`Is Valid`
        _)
      (:`Is Not Valid`
        (bind _returnvalue (`KismetMaterialLibrary.CreateDynamicMaterialInstance` (`self.M_Pixelation`)))
        (set `self.MI_Pixelation` _returnvalue)))
    (`PostProcessComponent.AddOrUpdateBlendable` (`self.BasePostProcess`) (`self.MI_Pixelation`) 1.0)
    (`MaterialInstanceDynamic.SetScalarParameterValue` (`self.MI_Pixelation`) "PixalationIntensity" (`self.PixelationValue`)))
  (return))

(fn `CreateRadiation`
  (params (bIsEnabled :type Boolean))
  (if bIsEnabled
    (`/Engine/EditorBlueprintResources/StandardMacros.IsValid` (`self.MI_Radiation`)
      (:`Is Valid`
        _)
      (:`Is Not Valid`
        (bind _returnvalue (`KismetMaterialLibrary.CreateDynamicMaterialInstance` (`self.M_Radiation`)))
        (set `self.MI_Radiation` _returnvalue)))
    (`PostProcessComponent.AddOrUpdateBlendable` (`self.BasePostProcess`) (`self.MI_Radiation`) 1.0)
    (`MaterialInstanceDynamic.SetScalarParameterValue` (`self.MI_Radiation`) "NoiseRadius" (`self.RadiationNoiseRadius`))
    (`MaterialInstanceDynamic.SetScalarParameterValue` (`self.MI_Radiation`) "RadiationRadius" (`self.RadiationRadius`))
    (`MaterialInstanceDynamic.SetScalarParameterValue` (`self.MI_Radiation`) "NoiseItensity" (`self.RadiationNoiseIntensity`)))
  (return))

(fn `CreateWater`
  (params (bIsEnabled :type Boolean))
  (if bIsEnabled
    (`/Engine/EditorBlueprintResources/StandardMacros.IsValid` (`self.MI_Water`)
      (:`Is Valid`
        _)
      (:`Is Not Valid`
        (bind _returnvalue (`KismetMaterialLibrary.CreateDynamicMaterialInstance` (`self.M_Water`)))
        (set `self.MI_Water` _returnvalue)))
    (`PostProcessComponent.AddOrUpdateBlendable` (`self.BasePostProcess`) (`self.MI_Water`) 1.0)
    (`MaterialInstanceDynamic.SetScalarParameterValue` (`self.MI_Water`) "WaterSharpness" (`self.WaterSharpness`))
    (`MaterialInstanceDynamic.SetScalarParameterValue` (`self.MI_Water`) "WaterDistance" (`self.WaterDistance`))
    (`MaterialInstanceDynamic.SetScalarParameterValue` (`self.MI_Water`) "WaveDistance" (`self.WaveDistance`)))
  (return))

(fn `Setup`
  (bind _basepostprocess (`self.BasePostProcess`))
  (set `PostProcessComponent.bUnbound` (`self.Unbound`) _basepostprocess)
  (set `PostProcessComponent.Settings` (`self.PostProcessSettings`) _basepostprocess)
  (setmembers `PostProcessSettings` :`StructRef` (`PostProcessComponent.Settings` _basepostprocess))
  (return))

(fn `UserConstructionScript`
  (if (`self.bIsEnabled`)
    (`self.Setup`)
    (`self.CheckState`)))