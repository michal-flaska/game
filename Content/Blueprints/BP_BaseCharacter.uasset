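; Base player character Blueprint using Enhanced Input for movement, look, jump, crouch, run, slow walk and shooting; lean is an empty stub.
; BeginPlay adds the IMC_Base mapping context and prints a TestFunction result.
; Run and slow walk multiply current max speed by modifiers on press and divide on release.
; Shoot line-traces from the camera, ignoring "ST"-tagged actors, and only debug-draws and prints "Enemy"-tagged hits, applying no damage.
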(event `self.ReceiveBeginPlay`
  (`self.Initialize`)
  (bind _returnvalue (`/Game/Blueprints/BP_BaseFunctionLibrary.TestFunction` (`self.RunSpeedModifier`) (`self.SlowSpeedModifier`)))
  (`KismetSystemLibrary.PrintString` (`KismetStringLibrary.Conv_DoubleToString` _returnvalue)))

(event `self.ReceiveTick`
  (params (DeltaSeconds :type "Float (single-precision)")))

(event `EnhancedInput|/Game/Input/IA_Lean`
  (params (ActionValue :type Boolean) (ElapsedSeconds :type "Float (double-precision)") (TriggeredSeconds :type "Float (double-precision)") (InputAction :type "InputAction Object Reference" :default "/Game/Input/IA_Lean.IA_Lean")))

(event `EnhancedInput|/Game/Input/IA_Shoot`
  (params (ActionValue :type Boolean) (ElapsedSeconds :type "Float (double-precision)") (TriggeredSeconds :type "Float (double-precision)") (InputAction :type "InputAction Object Reference" :default "/Game/Input/IA_Shoot.IA_Shoot"))
  (:`Started`
    (`self.Shoot`)))

(event `EnhancedInput|/Game/Input/IA_Jump`
  (params (ActionValue :type Boolean) (ElapsedSeconds :type "Float (double-precision)") (TriggeredSeconds :type "Float (double-precision)") (InputAction :type "InputAction Object Reference" :default "/Game/Input/IA_Jump.IA_Jump"))
  (:`Triggered`
    (`self.Jump`)))

(event `EnhancedInput|/Game/Input/IA_SlowWalk`
  (params (ActionValue :type Boolean) (ElapsedSeconds :type "Float (double-precision)") (TriggeredSeconds :type "Float (double-precision)") (InputAction :type "InputAction Object Reference" :default "/Game/Input/IA_SlowWalk.IA_SlowWalk"))
  (:`Started`
    (`self.StartSlowWalk`))
  (:`Completed`
    (`self.StopSlowWalk`)))

(event `EnhancedInput|/Game/Input/IA_Run`
  (params (ActionValue :type Boolean) (ElapsedSeconds :type "Float (double-precision)") (TriggeredSeconds :type "Float (double-precision)") (InputAction :type "InputAction Object Reference" :default "/Game/Input/IA_Run.IA_Run"))
  (:`Started`
    (`self.StartRunning`))
  (:`Completed`
    (`self.StopRunning`)))

(event `EnhancedInput|/Game/Input/IA_Crouch`
  (params (ActionValue :type Boolean) (ElapsedSeconds :type "Float (double-precision)") (TriggeredSeconds :type "Float (double-precision)") (InputAction :type "InputAction Object Reference" :default "/Game/Input/IA_Crouch.IA_Crouch"))
  (:`Triggered`
    (`self.StopJumping`)
    (`self.Crouch`))
  (:`Completed`
    (`self.UnCrouch`)))

(event `EnhancedInput|/Game/Input/IA_Look`
  (params (ActionValue :type "Vector2D Structure") (ElapsedSeconds :type "Float (double-precision)") (TriggeredSeconds :type "Float (double-precision)") (InputAction :type "InputAction Object Reference" :default "/Game/Input/IA_Look.IA_Look"))
  (:`Triggered`
    (`self.Look` ActionValue_X ActionValue_Y)))

(event `EnhancedInput|/Game/Input/IA_Move`
  (params (ActionValue :type "Vector2D Structure") (ElapsedSeconds :type "Float (double-precision)") (TriggeredSeconds :type "Float (double-precision)") (InputAction :type "InputAction Object Reference" :default "/Game/Input/IA_Move.IA_Move"))
  (:`Triggered`
    (`self.Move` ActionValue_X ActionValue_Y)))

(fn `Initialize`
  (`EnhancedInputSubsystemInterface.AddMappingContext` (pcsubsystem `EnhancedInputLocalPlayerSubsystem` (`GameplayStatics.GetPlayerController` 0)) "/Game/Input/IMC_Base.IMC_Base" 0 (struct)))

(fn `Look`
  (params (X :type "Float (single-precision)") (Y :type "Float (single-precision)"))
  (`self.AddControllerYawInput` X)
  (`self.AddControllerPitchInput` Y))

(fn `Move`
  (params (X :type "Float (single-precision)") (Y :type "Float (single-precision)"))
  (`self.AddMovementInput` (`self.GetActorRightVector`) X)
  (`self.AddMovementInput` (`self.GetActorForwardVector`) Y))

(fn `Shoot`
  (bind _returnvalue (`GameplayStatics.GetPlayerCameraManager` 0))
  (bind _returnvalue_2 (`SceneComponent.K2_GetComponentLocation` (`Actor.RootComponent` _returnvalue)))
  (bind _outactors (`GameplayStatics.GetAllActorsWithTag` "ST"))
  (bind _outhit (`KismetSystemLibrary.LineTraceSingle` _returnvalue_2 (+ _returnvalue_2 (* (`SceneComponent.GetForwardVector` (`Actor.RootComponent` _returnvalue)) 50000.0)) "TraceTypeQuery1" false _outactors "ForDuration"))
  (if (`self.ActorHasTag` (`.HitActor` (`GameplayStatics.BreakHitResult` _outhit)) "Enemy")
    (`KismetSystemLibrary.DrawDebugSphere` (`.Location` (`GameplayStatics.BreakHitResult` _outhit)) 100.0 12 (struct :`R` 1.0 :`B` 1.0 :`A` 1.0) 10.0 2.0)
    (`KismetSystemLibrary.PrintString` (`KismetSystemLibrary.GetDisplayName` (`.HitActor` (`GameplayStatics.BreakHitResult` _outhit))))))

(fn `StartRunning`
  (bind _charactermovement (`self.CharacterMovement`))
  (set `CharacterMovementComponent.MaxWalkSpeed` (* (`MovementComponent.GetMaxSpeed` _charactermovement) (`self.RunSpeedModifier`)) _charactermovement))

(fn `StartSlowWalk`
  (bind _charactermovement (`self.CharacterMovement`))
  (set `CharacterMovementComponent.MaxWalkSpeed` (* (`MovementComponent.GetMaxSpeed` _charactermovement) (`self.SlowSpeedModifier`)) _charactermovement))

(fn `StopRunning`
  (bind _charactermovement (`self.CharacterMovement`))
  (set `CharacterMovementComponent.MaxWalkSpeed` (/ (`MovementComponent.GetMaxSpeed` _charactermovement) (`self.RunSpeedModifier`)) _charactermovement))

(fn `StopSlowWalk`
  (bind _charactermovement (`self.CharacterMovement`))
  (set `CharacterMovementComponent.MaxWalkSpeed` (/ (`MovementComponent.GetMaxSpeed` _charactermovement) (`self.SlowSpeedModifier`)) _charactermovement))

(fn `UserConstructionScript`)